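; HealthLight is a health pickup that restores a TwinStickPawn to its default health on overlap.
; A looping timer rapidly randomizes the point light's color within reddish tones to create a flicker.
; On pawn overlap it resets health, then a DoOnce plays the pickup sound, clears HasHealthLight on the first GrowerSpawner found and destroys the actor.
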(event `self.ReceiveBeginPlay`
  (`KismetSystemLibrary.K2_SetTimer` null "ChangeLight" 0.05 true))

(event `self.ReceiveTick`
  (params (DeltaSeconds :type "Float (single-precision)")))

(event `ChangeLight`
  (`LightComponent.SetLightColor` (`self.PointLight`) (make `LinearColor` (`KismetMathLibrary.RandomFloatInRange` 0.8 1.0) (`KismetMathLibrary.RandomFloatInRange` 0.0 0.35) (`KismetMathLibrary.RandomFloatInRange` 0.0 0.35) 1.0) false))

(event `self.ReceiveActorBeginOverlap`
  (params (OtherActor :type "Actor Object Reference"))
  (bind _astwin_stick_pawn (cast `/Game/TwinStickBP/Blueprints/TwinStickPawn` OtherActor))
  (set `/Game/TwinStickBP/Blueprints/TwinStickPawn.health` (`/Game/TwinStickBP/Blueprints/TwinStickPawn.defaultHealth` _astwin_stick_pawn) _astwin_stick_pawn)
  (`/Engine/EditorBlueprintResources/StandardMacros.DoOnce` false
    (:`Completed`
      (`GameplayStatics.PlaySound2D` "/Game/Sounds/healthUp.healthUp" 1.3 1.0 0.3 null null)
      (bind _outactors (`GameplayStatics.GetAllActorsOfClass` "/Game/Blueprints/GrowerSpawner.GrowerSpawner_C"))
      (set `/Game/Blueprints/GrowerSpawner.hasHealthLight` false (`|GetArrayItem` _outactors))
      (`self.K2_DestroyActor`))))

(fn `UserConstructionScript`)