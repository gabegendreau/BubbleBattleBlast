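; Grower is a twin-stick game target that swells each time a projectile hits it and pops after 30 hits.
; On BeginPlay it gets a random color through a dynamic material, and a timeline drives its point light intensity.
; Collision hits identify projectiles by object name substring, enlarge the mesh and add score to TwinStickGameMode.
; The final hit plays a pop sound, increments the popped count, awards a bonus and destroys the actor.
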(event `self.ReceiveBeginPlay`
  (bind _returnvalue (`PrimitiveComponent.CreateDynamicMaterialInstance` (`self.Grower`) 0 "/Game/Materials/GrowerMat.GrowerMat" "None"))
  (`MaterialInstanceDynamic.SetVectorParameterValue` _returnvalue "Base Color" (make `LinearColor` (`KismetMathLibrary.RandomFloatInRange` 0.0 1.0) (`KismetMathLibrary.RandomFloatInRange` 0.0 1.0) (`KismetMathLibrary.RandomFloatInRange` 0.0 1.0) 0.7))
  (bind (_direction _intensity) (`Timeline|Timeline_0`)
    (:`Update`
      (`LightComponent.SetIntensity` (`self.PointLight`) (* _intensity (`self.intensityMultiplier`))))))

(event `self.Collision.OnComponentHit`
  (params (HitComponent :type "PrimitiveComponent Object Reference") (OtherActor :type "Actor Object Reference") (OtherComp :type "PrimitiveComponent Object Reference") (NormalImpulse :type "Vector Structure") (Hit :type "HitResult Structure (by ref)"))
  (bind _grower (`self.Grower`))
  (if (`KismetStringLibrary.Contains` (`KismetSystemLibrary.GetObjectName` OtherActor) "projectile")
    (`SceneComponent.SetWorldScale3D` _grower (+ (`SceneComponent.K2_GetComponentScale` _grower) (0.2 0.2 0.2)))
    (`/Engine/EditorBlueprintResources/StandardMacros.IncrementInt` (`self.numHits`)
      (:`  `
        (bind _astwin_stick_game_mode (cast `/Game/TwinStickBP/Blueprints/TwinStickGameMode` (`GameplayStatics.GetGameMode`)))
        (set `/Game/TwinStickBP/Blueprints/TwinStickGameMode.score` (+ 10 (`/Game/TwinStickBP/Blueprints/TwinStickGameMode.score` _astwin_stick_game_mode)) _astwin_stick_game_mode)
        (if (>= (`self.numHits`) 30)
          (`GameplayStatics.PlaySound2D` "/Game/Sounds/pop.pop" 1.5 1.0 0.0 null null)
          (bind _astwin_stick_game_mode_2 (cast `/Game/TwinStickBP/Blueprints/TwinStickGameMode` (`GameplayStatics.GetGameMode`)))
          (`/Game/TwinStickBP/Blueprints/TwinStickGameMode.incPopped` _astwin_stick_game_mode_2)
          (set `/Game/TwinStickBP/Blueprints/TwinStickGameMode.score` (+ 100 (`/Game/TwinStickBP/Blueprints/TwinStickGameMode.score` _astwin_stick_game_mode)) _astwin_stick_game_mode)
          (`self.K2_DestroyActor`))))))

(fn `UserConstructionScript`)