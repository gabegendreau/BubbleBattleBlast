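; GrowerSpawner is an actor that populates its SpawnZone bounds with Grower actors and a one-time HealthLight pickup for the twin-stick player.
; BeginPlay spawns an initial batch of Growers, then a looping named timer keeps adding more at random X/Y points at a fixed height.
; Tick watches the player pawn's health and spawns a single HealthLight the first time it drops to a sixth of default, latched by HasHealthLight.
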(event `self.ReceiveTick`
  (params (DeltaSeconds :type "Float (single-precision)"))
  (if (not (`self.hasHealthLight`))
    (bind _astwin_stick_pawn (cast `/Game/TwinStickBP/Blueprints/TwinStickPawn` (`GameplayStatics.GetPlayerPawn` 0)))
    (if (<= (`/Game/TwinStickBP/Blueprints/TwinStickPawn.health` _astwin_stick_pawn) (/ (`/Game/TwinStickBP/Blueprints/TwinStickPawn.defaultHealth` _astwin_stick_pawn) 6.0))
      (`self.SpawnHealthLight`))))

(event `SpawnHealthLight`
  (bind (_origin _boxextent) (`KismetSystemLibrary.GetComponentBounds` (`self.SpawnZone`)))
  (bind (_returnvalue_x _returnvalue_y) (`KismetMathLibrary.BreakVector` (`KismetMathLibrary.RandomPointInBoundingBox` _origin _boxextent)))
  (set `self.hasHealthLight` true)
  (`|SpawnActorFromClass` "/Game/Blueprints/HealthLight.HealthLight_C" (`KismetMathLibrary.MakeTransform` (`KismetMathLibrary.MakeVector` _returnvalue_x _returnvalue_y 231.725967)) "Undefined" "OverrideRootScale" null null))

(event `self.ReceiveBeginPlay`
  (for _ (range 1 8)
    (`self.SpawnGrower`))
  (`KismetSystemLibrary.K2_SetTimer` null "SpawnGrower" 7.0 true))

(event `SpawnGrower`
  (bind (_origin _boxextent) (`KismetSystemLibrary.GetComponentBounds` (`self.SpawnZone`)))
  (bind (_returnvalue_x _returnvalue_y) (`KismetMathLibrary.BreakVector` (`KismetMathLibrary.RandomPointInBoundingBox` _origin _boxextent)))
  (`|SpawnActorFromClass` "/Game/Blueprints/Grower.Grower_C" (`KismetMathLibrary.MakeTransform` (`KismetMathLibrary.MakeVector` _returnvalue_x _returnvalue_y 231.725967)) "Undefined" "OverrideRootScale" null null))

(fn `UserConstructionScript`)